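; BP_Texture is a Blueprint tool that bakes a material into a static texture asset.
; BakeTexture prints a status message, then, if both the render target and material are valid, draws the material into the render target.
; It saves that result as a Texture2D named TextureFromRenderTarget through an editor-only call, so the baking works only in the editor.
; The construction script is empty.
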(fn ConstructionScript)

(fn BakeTexture
  (Development|PrintString "Baking Textures")
  (if (and (Utilities|IsValid (Variables|RenderTargetSettings|GetRenderTargetToDraw)) (Utilities|IsValid (Variables|RenderTargetSettings|GetMaterialToDrawFrom)))
    (Rendering|DrawMaterialtoRenderTarget (Variables|RenderTargetSettings|GetRenderTargetToDraw) (Variables|RenderTargetSettings|GetMaterialToDrawFrom))
    (Class|KismetRenderingLibrary|RenderTargetCreateStaticTexture2DEditorOnly (Variables|RenderTargetSettings|GetRenderTargetToDraw) "TextureFromRenderTarget" "TC_Default" "TMGS_FromTextureGroup")))